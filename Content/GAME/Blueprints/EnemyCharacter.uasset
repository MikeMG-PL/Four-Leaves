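; Enemy character Blueprint that roams at random and shoots at the player when it sees them.
; From BeginPlay it loops AIMoveTo to random reachable points nearby, restarting only when a move succeeds.
; PawnSensing turns it by yaw toward the player and spawns EnemyBullet at BulletSpawn, aimed on all axes and throttled by a ShootDelay flag.
; Tick prints its movement speed.
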(event OnSeePawn(PawnSensing)
  (params (Pawn :type Pawn%20Object%20Reference))
  (bind _returnvalue (Transformation|GetActorLocation))
  (bind _bulletspawn (Variables|Default|GetBulletSpawn))
  (bind _asthe_power_of_four_leaves_character (Utilities|Casting|CastToThePowerOfFourLeavesCharacter Pawn))
  (Utilities|FlowControl|Sequence
    (:then_0
      (Transformation|SetActorRotation (Math|Rotator|MakeRotator 0.0 0.0 (.yaw (Math|Rotator|FindLookatRotation _returnvalue (Transformation|GetActorLocation _asthe_power_of_four_leaves_character))))))
    (:then_1
      (if (Variables|Default|GetShootDelay)
        (Game|SpawnActorfromClass "/Game/GAME/Blueprints/EnemyBullet.EnemyBullet_C" (Math|Transform|MakeTransform (Transformation|GetWorldLocation _bulletspawn) (Math|Rotator|FindLookatRotation _returnvalue (Transformation|GetActorLocation _asthe_power_of_four_leaves_character)) (Transformation|GetWorldScale _bulletspawn)) "Undefined" 0 0)
        ;[1 1 1] Delay between two next consecutive shoots
        (Variables|Default|SetShootDelay false)
        (Utilities|FlowControl|Delay 1.0)
        (Variables|Default|SetShootDelay true)))))

(event Custom|Random%20Roam
  (AI|AIMoveTo self (.RandomLocation (AI|Navigation|GetRandomReachablePointinRadius (Transformation|GetActorLocation) 6e+02 0 0)) 0 5.0 false
    (:OnSuccess
      (CallFunction|RandomRoam))))

(event EventBeginPlay
  (CallFunction|RandomRoam))

(event Collision|EventActorBeginOverlap
  (params (OtherActor :type Actor%20Object%20Reference)))

(event EventTick
  (params (DeltaSeconds :type Float%20%28single-precision%29))
  (Development|PrintString (Utilities|String|ToString(Float) (Math|Vector|VectorLength (Variables|/Script/Engine.MovementComponent|GetVelocity (Pawn|GetMovementComponent))))))

(fn ConstructionScript)