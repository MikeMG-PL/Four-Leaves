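; Player life component that shows the current number of lives on a HUD widget.
; On BeginPlay it creates the HUD, adds it to the viewport and keeps a reference to it.
; Each Tick it loops over the HUD's image array, showing images with an index below CurrentNumberOfLifes and hiding the rest, so the display is polled rather than event-driven.
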(event EventBeginPlay
  (UserInterface|CreateWidget "/Game/GAME/UI/HUD.HUD_C")
  (bind _returnvalue (UserInterface|CreateWidget "/Game/GAME/UI/HUD.HUD_C"))
  (UserInterface|Viewport|AddtoViewport _returnvalue 0)
  (Variables|Default|SetHUD _returnvalue))

(event EventTick
  (params (DeltaSeconds :type Float%20%28single-precision%29))
  (for (_array_element _array_index) (Variables|/Game/GAME/UI/HUD.HUD_C|GetImages (Variables|Default|GetHUD))
    (if (< _array_index (Variables|Default|GetCurrentNumberOfLifes))
      (Variables|/Script/UMG.Widget|SetVisibility _array_element "Visible")
      (else
        (Variables|/Script/UMG.Widget|SetVisibility _array_element "Hidden")))))