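; DestructiblePlank is an actor that breaks when the player character dashes into it.
; On overlap it casts the other actor to BP_ThePowerOfFourLeavesCharacter and checks its IsDashing flag.
; If dashing, it spawns the class of its DestroyedActor variable at its own location and rotation with unit scale, prints the spawned actor's name, then destroys itself.
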(event EventBeginPlay)

(event Collision|EventActorBeginOverlap
  (params (OtherActor :type Actor%20Object%20Reference))
  (bind _returnvalue (Transformation|GetActorTransform))
  (bind _asbp_the_power_of_four_leaves_character (Utilities|Casting|CastToBP_ThePowerOfFourLeavesCharacter OtherActor))
  (if (Utilities|IsValid _asbp_the_power_of_four_leaves_character)
    (if (Variables|/Game/GAME/Blueprints/BP_ThePowerOfFourLeavesCharacter.BP_ThePowerOfFourLeavesCharacter_C|GetIsDashing _asbp_the_power_of_four_leaves_character)
      (bind _returnvalue_2 (Game|SpawnActorfromClass (Utilities|GetClass (Variables|Default|GetDestroyedActor)) (Math|Transform|MakeTransform (.location _returnvalue) (.rotation _returnvalue)) "Undefined" 0 0))
      (Development|PrintString (Utilities|GetDisplayName _returnvalue_2))
      (Actor|DestroyActor))))

(event EventTick
  (params (DeltaSeconds :type Float%20%28single-precision%29)))

(fn ConstructionScript)