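; Player character Blueprint that adds a dash ability, triggered by the IA_Dash Enhanced Input action.
; The dash gives a small upward launch, then after a brief delay launches the character strongly along its forward vector.
; A Cooldown flag, set after the forward launch and cleared by a timed delay, gates reuse.
; IsDashing is set on dash start and cleared on landing only while the cooldown is active.
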(event Input|EnhancedActionEvents|EnhancedInputActionIA_Dash
  (params (ActionValue :type Boolean) (ElapsedSeconds :type Float%20%28double-precision%29) (TriggeredSeconds :type Float%20%28double-precision%29) (InputAction :type Input%20Action%20Object%20Reference :default "/Game/GAME/Input/IA_Dash.IA_Dash"))
  (:Triggered
    (if (not (Variables|Default|GetCooldown))
      (Variables|Default|SetIsDashing true)
      (Character|LaunchCharacter "0.000000,0.000000,200.000000" false false)
      (Utilities|FlowControl|Delay 0.1)
      (Character|LaunchCharacter (* (Math|Vector|GetForwardVector (Transformation|GetActorRotation)) (Math|Float|MakeLiteralFloat 2.5e+03)) false false)
      (Variables|Default|SetCooldown true)
      (Utilities|FlowControl|Delay 2.0)
      (Variables|Default|SetCooldown false))))

(event EventOnLanded
  (params (Hit :type Hit%20Result%20Structure%20%28by%20ref%29))
  (if (Variables|Default|GetCooldown)
    (Variables|Default|SetIsDashing false)))

(fn ConstructionScript)