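; Line is an actor with a Burst effect and an optional blocking volume, both driven by the state of other referenced actors.
; When the Lepricon flag is set, it switches Burst off at BeginPlay and activates it on Tick once the Lepricon reference is no longer valid.
; When the door flag is set, Tick destroys the BlockingVolume once the Door is gone.
; Both triggers poll validity every frame rather than binding to destruction events.
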(event EventBeginPlay
  (if (Variables|Default|GetActivateOnLepriconDeath)
    (Components|Activation|Deactivate (Variables|Default|GetBurst))))

(event Collision|EventActorBeginOverlap
  (params (OtherActor :type Actor%20Object%20Reference)))

(event EventTick
  (params (DeltaSeconds :type Float%20%28single-precision%29))
  (bind _blockingvolume (Variables|Default|GetBlockingVolume))
  (Utilities|FlowControl|Sequence
    (:then_0
      (if (Variables|Default|GetActivateOnLepriconDeath)
        (if (not (Utilities|IsValid (Variables|Default|GetLepricon)))
          (Components|Activation|Activate (Variables|Default|GetBurst) false))))
    (:then_1
      (if (Variables|Default|GetDisactivateOnDoorDestroy)
        (if (not (Utilities|IsValid (Variables|Default|GetDoor)))
          (Utilities|IsValid _blockingvolume
            (:Is%20Valid
              (Actor|DestroyActor _blockingvolume))))))))

(fn ConstructionScript)